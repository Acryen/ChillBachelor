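; BP_EnemyCharacter is an enemy character Blueprint with empty BeginPlay and construction script.
; Its only logic is an unconnected death sequence that never runs.
; That sequence plays AM_Death on the mesh and, on blend out, switches to ragdoll physics.
; The mesh is set to block all channels except Visibility, Pawn and Camera, which it ignores.
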(event EventBeginPlay)

(fn ConstructionScript)